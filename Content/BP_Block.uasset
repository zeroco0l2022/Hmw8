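; BP_Block is a destructible block that loses health each time it receives a Hit event and can drop a bonus.
; TakeDamage decrements the clamped health, tints the Geometry Collection red and reports when the minimum is reached.
; Death switches the collection and box to physics bodies, clears tags, rolls a BP_Bonus spawn, then destroys the actor after a short random delay.
; OnTarget exposes the scene root.
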(event Custom|Death
  ;[1 0.164 0] DeathEvent
  (CallFunction|OnDeath)
  (CallFunction|Bonus)
  (Utilities|FlowControl|Delay (Math|Random|RandomFloatinRange 0.4 1.0))
  (Actor|DestroyActor))

(event EventBeginPlay
  ;[0.02061 1 0.1526] BeginPlay
  (Variables|Default|SetHealth 2))

(event Collision|EventHit
  (params (MyComp :type Primitive%20Component%20Object%20Reference) (Other :type Actor%20Object%20Reference) (OtherComp :type Primitive%20Component%20Object%20Reference) (bSelfMoved :type Boolean) (HitLocation :type Vector :default "0, 0, 0") (HitNormal :type Vector :default "0, 0, 0") (NormalImpulse :type Vector :default "0, 0, 0") (Hit :type Hit%20Result%20Structure%20%28by%20ref%29))
  ;[1 0.9385 0] EventHit
  (if (CallFunction|TakeDamage)
    (CallFunction|Death)))

(fn ConstructionScript)

(fn OnDeath
  (bind _geometrycollection (Variables|Default|GetGeometryCollection))
  (Physics|SetSimulatePhysics _geometrycollection true)
  (Collision|SetCollisionObjectType _geometrycollection "ECC_PhysicsBody")
  (Utilities|Array|Clear (Variables|Actor|GetTags))
  (Collision|SetCollisionObjectType (Variables|Default|GetBox) "ECC_PhysicsBody"))

(fn TakeDamage
  (bind _result (Math|Integer|DecrementInt (Variables|Default|GetHealth))
    (:%20%20
      (Variables|Default|SetHealth (Math|Integer|Max(Integer) _result (Variables|Default|GetMinHealth)))
      (Rendering|Material|SetMaterial (Variables|Default|GetGeometryCollection) 0 "/AnimationSharing/AnimSharingRed.AnimSharingRed")
      (return (<= (Variables|Default|GetHealth) (Variables|Default|GetMinHealth))))))

(fn Bonus
  (if (Math|Random|RandomBoolwithWeight 0.5)
    (Game|SpawnActorfromClass "/Game/BP_Bonus.BP_Bonus_C" (Math|Transform|MakeTransform (Transformation|GetActorLocation) "0, 0, 0" "1.000000,1.000000,1.000000") "Undefined" "MultiplyWithRoot" 0 0)))

(fn OnTarget
  (return (Variables|Default|GetDefaultSceneRoot)))