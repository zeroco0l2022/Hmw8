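; A bouncing ball projectile that moves at constant speed and fires OnDeath, then destroys itself, on entering a KillZVolume.
; On hit, it reflects off the surface, adds the hit actor's velocity and renormalizes in 2D to Speed.
; Each bounce picks a new homing target by line-tracing an alternating, widening fan around its velocity for BPI_Targetable actors, skipping the previous target.
; The search traces leave debug drawing enabled.
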(event OnProjectileBounce(ProjectileMovement)
  (params (ImpactResult :type Hit%20Result%20Structure%20%28by%20ref%29) (ImpactVelocity :type Vector%20%28by%20ref%29 :default "0, 0, 0"))
  ;[1 0.1118 0.07198] SearchHomingTarget
  (Variables|Default|SetLastHomingTarget (Variables|/Script/Engine.ProjectileMovementComponent|GetHomingTargetComponent (Variables|Default|GetProjectileMovement)))
  (Variables|/Script/Engine.ProjectileMovementComponent|SetHomingTargetComponent (Variables|Default|GetProjectileMovement) (CallFunction|FindHomingTarget)))

(event Collision|EventActorBeginOverlap
  (params (OtherActor :type Actor%20Object%20Reference))
  ;[0.1583 0.2487 1] KillZ
  (Utilities|Casting|CastToKillZVolume OtherActor)
  (Default|CallOnDeath)
  (Actor|DestroyActor))

(event EventBeginPlay
  (bind _projectilemovement (Variables|Default|GetProjectileMovement))
  ;[0 1 0.739] Begin Play/Set Speed
  (bind _output_get (Variables|/Script/Engine.ProjectileMovementComponent|SetInitialSpeed _projectilemovement (Variables|Default|GetSpeed)))
  (Variables|/Script/Engine.ProjectileMovementComponent|SetMaxSpeed _projectilemovement _output_get)
  (Variables|/Script/Engine.ProjectileMovementComponent|SetHomingAccelerationMagnitude _projectilemovement 2e+04))

(event Collision|EventHit
  (params (MyComp :type Primitive%20Component%20Object%20Reference) (Other :type Actor%20Object%20Reference) (OtherComp :type Primitive%20Component%20Object%20Reference) (bSelfMoved :type Boolean) (HitLocation :type Vector :default "0, 0, 0") (HitNormal :type Vector :default "0, 0, 0") (NormalImpulse :type Vector :default "0, 0, 0") (Hit :type Hit%20Result%20Structure%20%28by%20ref%29))
  ;[0.9101 0.2067 1] HitReaction
  (Variables|/Script/Engine.MovementComponent|SetVelocity (Variables|Default|GetProjectileMovement) (CallFunction|CalcNormalizedDirection Other HitNormal)))

(fn ConstructionScript)

(fn CalcNormalizedDirection
  (params (OtherActor :type Actor%20Object%20Reference) (HitNormal :type Vector))
  (return (* (Class|KismetMathLibrary|VectorNormal2D (+ (Transformation|GetVelocity OtherActor) (Math|Vector|GetReflectionVector (Transformation|GetVelocity) HitNormal)) 0.0001) (Variables|Default|GetSpeed))))

(fn FindHomingTarget
  (bind _returnvalue (Transformation|GetActorLocation))
  (bind _index (Utilities|FlowControl|ForLoopwithBreak 0 (LocalVariables|GetLastIndex) :!label _label)
    (:LoopBody
      (LocalVariables|SetAngle (* (LocalVariables|GetAngle) -1))
      (bind (_outhit _returnvalue_2) (Collision|LineTraceForObjects _returnvalue (+ _returnvalue (* (Math|Vector|RotateVector (Variables|/Script/Engine.MovementComponent|GetVelocity (Variables|Default|GetProjectileMovement)) (Math|Rotator|MakeRotator 0.0 0.0 (Math|Conversions|ToFloat(Integer) (* _index (/ (LocalVariables|GetAngle) (+ (LocalVariables|GetLastIndex) 1)))))) 2.5e+03)) (LocalVariables|GetObject%20Types) false 0 "Persistent" true "(R=1.000000,G=0.000000,B=0.000000,A=1.000000)" "(R=0.000000,G=1.000000,B=0.000000,A=1.000000)" 0.3))
      (if _returnvalue_2
        (if (Utilities|DoesObjectImplementInterface (.hitactor _outhit) "/Game/BPI_Targetable.BPI_Targetable_C")
          (bind _hometarget (Class|BPITargetable|OnTarget(Message) (.hitactor _outhit)))
          (if (!= (Variables|Default|GetLastHomingTarget) _hometarget)
            (Utilities|FlowControl|Sequence
              (:then_0
                (goto _label Break))
              (:then_1
                (return _hometarget)))))))))

(fn OnTarget)